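; Vehicle lane spawner that emits Vehicle_BP actors, passing each its facing, a chicken reference and one random speed chosen at BeginPlay.
; Tick accumulates time and spawns a vehicle at the spawner's transform after each re-randomized interval.
; BeginPlay also runs an initial spawn loop while ContinueCreatingVehicles holds, placing vehicles at a facing-dependent X offset.
; That loop computes random spacing and accumulated distance, but the spawn location does not use them.
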(event EventBeginPlay
  (Variables|Default|SetSpeed (Math|Random|RandomFloatinRange 3e+02 6e+02))
  (CallFunction|SetNewMaxTimeforSpawn)
  (CallFunction|SpawnInitialVehicle))

(event EventTick
  (params (DeltaSeconds :type Float%20%28single-precision%29))
  (bind _output_get (Variables|Default|SetTime%20Accumulation (+ DeltaSeconds (Variables|Default|GetTime%20Accumulation))))
  (if (>= _output_get (Variables|Default|GetTime%20Max%20for%20Spawn))
    (Variables|Default|SetTime%20Accumulation 0.0)
    (CallFunction|SetNewMaxTimeforSpawn)
    (Game|SpawnActorfromClass "/Game/Blueprints/Vehicle_BP.Vehicle_BP_C" (Transformation|GetActorTransform) "Undefined" 0 (Variables|Default|GetFacing%20Left) (Variables|Default|GetSpeed) (Variables|Default|GetChicken%20REF) 0)))

(fn ConstructionScript)

(fn SetNewMaxTimeforSpawn
  (Variables|Default|SetTime%20Max%20for%20Spawn (Math|Random|RandomFloatinRange 2.0 5.0)))

(fn SpawnInitialVehicle
  (bind _returnvalue (Transformation|GetActorLocation))
  (bind _returnvalue_2 (Math|Random|RandomFloatinRange 6e+02 1.2e+03))
  (bind _returnvalue_3 (Transformation|GetActorLocation))
  (if (Variables|Default|GetFacing%20Left)
    (LocalVariables|SetX%20Offset%20Initial (+ (.x _returnvalue) -6e+02))
    (else
      (LocalVariables|SetX%20Offset%20Initial (+ (.x _returnvalue) 6e+02))))
  (while (LocalVariables|GetContinue%20Creating%20Vehicles)
    (LocalVariables|SetX%20Offset%20Accumulation _returnvalue_2)
    (LocalVariables|SetDistance%20Accumulation (+ _returnvalue_2 (LocalVariables|GetDistance%20Accumulation)))
    (if (Variables|Default|GetFacing%20Left)
      (LocalVariables|SetX%20Offset%20Accumulation (* (LocalVariables|GetX%20Offset%20Accumulation) -1.0)))
    (Game|SpawnActorfromClass "/Game/Blueprints/Vehicle_BP.Vehicle_BP_C" (Math|Transform|MakeTransform (Math|Vector|MakeVector (LocalVariables|GetX%20Offset%20Initial) (.y _returnvalue_3) (.z _returnvalue_3))) "Undefined" 0 (Variables|Default|GetFacing%20Left) (Variables|Default|GetSpeed) (Variables|Default|GetChicken%20REF) 0)))