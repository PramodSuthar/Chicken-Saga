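; Grass row Blueprint that builds a strip of terrain with obstacles and landing nodes on BeginPlay.
; It spawns three floor pieces, optionally meant to darken, and dark outer prop groups on both sides, where the random rock check never passes, leaving only bushes.
; Each of nine inner slots randomly gets a bush or rock, or a landing node with a coin attempt; clear columns always stay open.
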(event EventBeginPlay
  (CallFunction|CreateGrassFloors)
  (CallFunction|CreateOuterBushesandRocks)
  (CallFunction|ConstructLandingNodes))

(fn ConstructionScript
  (|CallParentFunction))

(fn ReduceGrassColor
  (params (Current%20Floor :type Floor%20BP%20Object%20Reference))
  (bind _material_instance (Variables|/Game/Blueprints/Floor_BP.Floor_BP_C|GetMaterial%20Instance Current%20Floor))
  (bind _returnvalue (Rendering|Material|GetVectorParameterValue _material_instance "darkness" :!class /Script/Engine.MaterialInstanceDynamic))
  (Rendering|Material|SetVectorParameterValue _material_instance "" (Math|Conversions|ToLinearColor(Float) (- (.R (Utilities|Struct|BreakLinearColor _returnvalue)) 0.3)) :!class /Script/Engine.MaterialInstanceDynamic))

(fn CreateGrassFloors
  (bind (_transform_left _transform_mid _transform_right) (CallFunction|CalculateFloorTransform))
  (bind _returnvalue (Game|SpawnActorfromClass "/Game/Blueprints/Floor_BP.Floor_BP_C" _transform_left "Undefined" 0 0 false 0 0))
  (bind _output_get (Variables|Default|SetLeft%20Floor _returnvalue))
  (bind _returnvalue_2 (Game|SpawnActorfromClass "/Game/Blueprints/Floor_BP.Floor_BP_C" _transform_mid "Undefined" 0 0 true 0 0))
  (bind _output_get_2 (Variables|Default|SetCenter%20Floor _returnvalue_2))
  (bind _returnvalue_3 (Game|SpawnActorfromClass "/Game/Blueprints/Floor_BP.Floor_BP_C" _transform_right "Undefined" 0 0 false 0 0))
  (bind _output_get_3 (Variables|Default|SetRight%20Floor _returnvalue_3))
  (if (Variables|Default|GetDarker%20Grass)
    (CallFunction|ReduceGrassColor _output_get)
    (CallFunction|ReduceGrassColor _output_get_2)
    (CallFunction|ReduceGrassColor _output_get_3)))

(fn CreateSingleGroupOfOuterBushesandRocks
  (params (Current%20Outlier%20Position%20X%20in%20 :type Float%20%28single-precision%29))
  (bind _returnvalue (Transformation|GetActorLocation))
  (bind _props (Variables|Default|GetProps))
  (LocalVariables|SetCurrent%20X Current%20Outlier%20Position%20X%20in%20)
  (for _index (range 0 8)
    (if (> (Math|Random|RandomInteger 3) 2)
      (bind _returnvalue_2 (Game|SpawnActorfromClass "/Game/Blueprints/Rock_BP.Rock_BP_C" (Math|Transform|MakeTransform (Math|Vector|MakeVector (LocalVariables|GetCurrent%20X) (.y _returnvalue) (.z _returnvalue))) "Undefined" 0 true 0))
      (Utilities|Array|Add _props _returnvalue_2)
      (else
        (bind _returnvalue_3 (Game|SpawnActorfromClass "/Game/Blueprints/Bush_BP.Bush_BP_C" (Math|Transform|MakeTransform (Math|Vector|MakeVector (LocalVariables|GetCurrent%20X) (.y _returnvalue) (.z _returnvalue))) "Undefined" 0 true 0))
        (Utilities|Array|Add _props _returnvalue_3)))
    (LocalVariables|SetCurrent%20X (+ (LocalVariables|GetCurrent%20X) 2e+02))))

(fn CreateOuterBushesandRocks
  (CallFunction|CreateSingleGroupOfOuterBushesandRocks -2.6e+03)
  (CallFunction|CreateSingleGroupOfOuterBushesandRocks 1e+03))

(fn CheckifinClearColumns
  (if (== (Variables|Default|GetCurrent%20X%20Position%20for%20Landing%20Node) (Variables|Default|GetClear%20Col%20Pos%20X1))
    _
    (elif (== (Variables|Default|GetCurrent%20X%20Position%20for%20Landing%20Node) (Variables|Default|GetClear%20Col%20Pos%20X2))
      _
      (elif (== (Variables|Default|GetCurrent%20X%20Position%20for%20Landing%20Node) (Variables|Default|GetClear%20Col%20Pos%20X3))
        _
        (else
          (return false)))))
  (return true))

(fn CreateBushorRock
  (bind _props (Variables|Default|GetProps))
  (if (Math|Random|RandomBool)
    (bind _returnvalue (Game|SpawnActorfromClass "/Game/Blueprints/Bush_BP.Bush_BP_C" (Math|Transform|MakeTransform (Math|Vector|MakeVector (Variables|Default|GetCurrent%20X%20Position%20for%20Landing%20Node) (.y (Transformation|GetActorLocation)) (Variables|Default|GetCurrent%20Z%20Position%20for%20Landing%20Node))) "Undefined" 0 false 0))
    (Utilities|Array|Add _props _returnvalue)
    (else
      (bind _returnvalue_2 (Game|SpawnActorfromClass "/Game/Blueprints/Rock_BP.Rock_BP_C" (Math|Transform|MakeTransform (Math|Vector|MakeVector (Variables|Default|GetCurrent%20X%20Position%20for%20Landing%20Node) (.y (Transformation|GetActorLocation)) (Variables|Default|GetCurrent%20Z%20Position%20for%20Landing%20Node))) "Undefined" 0 false 0))
      (Utilities|Array|Add _props _returnvalue_2)))
  (Variables|Default|SetCurrent%20X%20Position%20for%20Landing%20Node (+ (Variables|Default|GetCurrent%20X%20Position%20for%20Landing%20Node) 2e+02)))

(fn ConstructLandingNodes
  (for _index (range 0 8)
    (if (== (Math|Random|RandomIntegerinRange 0 6) 0)
      (bind _in_clear_column (CallFunction|CheckifinClearColumns))
      (if _in_clear_column
        (CallFunction|CreateCoinAttempt :!label _label)
        (CallFunction|ConstructLandingNode(FloorChunk) false)
        (else
          (CallFunction|CreateBushorRock)))
      (else
        (goto _label)))))