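; Water floor chunk that lays a river row from three Floor_BP pieces, plus landing nodes and optional lily pads or moving logs.
; Up to three lily pads sit at distinct clear-column positions and are destroyed with the chunk.
; Logs pre-fill the row, then Tick spawns more off one side, timed by the last log's length and a per-chunk random speed bonus.
; Tick also checks whether to destroy the chunk.
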(event EventBeginPlay
  (bind _self self)
  (bind (_transform_left _transform_mid _transform_right) (CallFunction|CalculateFloorTransform))
  (bind _returnvalue (Game|SpawnActorfromClass "/Game/Blueprints/Floor_BP.Floor_BP_C" _transform_left "Undefined" 0 2 false _self 0))
  (Variables|Default|SetLeft%20Floor _returnvalue)
  (bind _returnvalue_2 (Game|SpawnActorfromClass "/Game/Blueprints/Floor_BP.Floor_BP_C" _transform_mid "Undefined" 0 2 true _self 0))
  (Variables|Default|SetCenter%20Floor _returnvalue_2)
  (bind _returnvalue_3 (Game|SpawnActorfromClass "/Game/Blueprints/Floor_BP.Floor_BP_C" _transform_right "Undefined" 0 2 false _self 0))
  (Variables|Default|SetRight%20Floor _returnvalue_3)
  (CallFunction|ConstructLandingNodes)
  (if (Variables|Default|GetCreate%20Logs)
    (CallFunction|ConstructInitialLogs)))

(event Collision|EventActorBeginOverlap
  (params (OtherActor :type Actor%20Object%20Reference)))

(event EventTick
  (params (DeltaSeconds :type Float%20%28single-precision%29))
  (if (Variables|Default|GetCreate%20Logs)
    (CallFunction|ConstuctLogAttempt DeltaSeconds))
  (CallFunction|CheckifDestroyFloorChunk))

(event EventDestroyed
  (for _array_element (Variables|Default|GetLily%20Pads)
    (Actor|DestroyActor _array_element)))

(fn ConstructionScript
  (if (Variables|Default|GetCreate%20Logs)
    (Variables|Default|SetMax%20Create%20Log%20Time (Math|Random|RandomFloatinRange 0.0 1.0))
    (CallFunction|AddExtraLogSpeedRandom)))

(fn ConstructSingleLilyPad
  (params (Current%20X :type Float%20%28single-precision%29))
  (bind _returnvalue (Transformation|GetActorLocation))
  (if (not (== Current%20X -1.0))
    (bind _returnvalue_2 (Game|SpawnActorfromClass "/Game/Blueprints/LilyPad_BP.LilyPad_BP_C" (Math|Transform|MakeTransform (Math|Vector|MakeVector Current%20X (.y _returnvalue) (- (.z _returnvalue) 3e+01))) "Undefined" 0 0))
    (Utilities|Array|Add (Variables|Default|GetLily%20Pads) _returnvalue_2)))

(fn ConstructMultipleLilyPads
  (bind _current_clear_column_position_x3 (Variables|Default|GetCurrent%20Clear%20Column%20Position%20X3))
  (if (>= (Variables|Default|GetNumber%20of%20Lily%20Pads%20to%20Create) 1)
    (CallFunction|ConstructSingleLilyPad (Variables|Default|GetCurrent%20Clear%20Column%20Position%20X1))
    (if (>= (Variables|Default|GetNumber%20of%20Lily%20Pads%20to%20Create) 2)
      (if (not (== (Variables|Default|GetCurrent%20Clear%20Column%20Position%20X1) (Variables|Default|GetCurrent%20Clear%20Column%20Position%20X2)))
        (CallFunction|ConstructSingleLilyPad (Variables|Default|GetCurrent%20Clear%20Column%20Position%20X2))
        (if (>= (Variables|Default|GetNumber%20of%20Lily%20Pads%20to%20Create) 3)
          (if (not (or (== (Variables|Default|GetCurrent%20Clear%20Column%20Position%20X2) _current_clear_column_position_x3) (== _current_clear_column_position_x3 (Variables|Default|GetCurrent%20Clear%20Column%20Position%20X1))))
            (CallFunction|ConstructSingleLilyPad (Variables|Default|GetCurrent%20Clear%20Column%20Position%20X3))))))))

(fn ConstructLandingNodes
  (Variables|Default|SetCurrent%20Z%20Position%20for%20Landing%20Node -6e+01)
  (for _index (range 0 0)
    (CallFunction|ConstructLandingNode(FloorChunk) true))
  (if (Variables|Default|GetCreate%20Lilypads)
    (CallFunction|ConstructMultipleLilyPads)))

(fn ConstructLogs
  (params (Location%20X :type Float%20%28single-precision%29))
  (bind _returnvalue (Transformation|GetActorLocation))
  (bind _returnvalue_2 (Game|SpawnActorfromClass "/Game/Blueprints/Log_BP.Log_BP_C" (Math|Transform|MakeTransform (Math|Vector|MakeVector Location%20X (.y _returnvalue) (.z _returnvalue))) "Undefined" 0 (Math|Random|RandomIntegerinRange 1 3) (not (Variables|Default|GetCreate%20Logs%20Left)) (Variables|Default|GetExtra%20Log%20Speed%20Center) 0))
  (bind _output_get (Variables|Default|SetCurrent%20Log%20Created _returnvalue_2))
  (return _output_get))

(fn CalculateLogCreationOffsetNext
  (Utilities|IsValid (Variables|Default|GetCurrent%20Log%20Created)
    (:Is%20Valid
      (switch int (Variables|/Game/Blueprints/Log_BP.Log_BP_C|GetLength (Variables|Default|GetCurrent%20Log%20Created))
        (:1
          (return (Math|Random|RandomFloatinRange 4e+02 5e+02)))
        (:2
          (return (Math|Random|RandomFloatinRange 6e+02 7e+02)))
        (:3
          (return (Math|Random|RandomFloatinRange 8e+02 9e+02)))))
    (:Is%20Not%20Valid
      (return (Math|Random|RandomFloatinRange 0.0 1e+02)))))

(fn ConstructInitialLogs
  (if (Variables|Default|GetCreate%20Logs%20Left)
    (LocalVariables|SetLog%20Create%20X%20Pos -9e+02)
    (while (< (LocalVariables|GetLog%20Create%20X%20Pos) 9e+02)
      (bind _random_x_pos (CallFunction|CalculateLogCreationOffsetNext))
      (bind _output_get (LocalVariables|SetLog%20Create%20X%20Pos (+ _random_x_pos (LocalVariables|GetLog%20Create%20X%20Pos))))
      (CallFunction|ConstructLogs _output_get))
    (else
      (LocalVariables|SetLog%20Create%20X%20Pos 9e+02)
      (while (> (LocalVariables|GetLog%20Create%20X%20Pos) -9e+02)
        (bind _random_x_pos_2 (CallFunction|CalculateLogCreationOffsetNext))
        (bind _output_get_2 (LocalVariables|SetLog%20Create%20X%20Pos (- (LocalVariables|GetLog%20Create%20X%20Pos) _random_x_pos_2)))
        (CallFunction|ConstructLogs _output_get_2)))))

(fn AddExtraLogSpeedRandom
  (Variables|Default|SetExtra%20Log%20Speed%20Center (Math|Random|RandomFloatinRange 0.0 2e+02)))

(fn ConstuctLogAttempt
  (params (Delta%20Time :type Float%20%28single-precision%29))
  (bind _extra_log_speed_center (Variables|Default|GetExtra%20Log%20Speed%20Center))
  (bind _returnvalue (/ _extra_log_speed_center 4e+02))
  (bind _output_get (Variables|Default|SetCurrent%20Create%20Log%20Time (+ Delta%20Time (Variables|Default|GetCurrent%20Create%20Log%20Time))))
  (if (>= _output_get (Variables|Default|GetMax%20Create%20Log%20Time))
    (if (Variables|Default|GetCreate%20Logs%20Left)
      (CallFunction|ConstructLogs -2.8e+03)
      (else
        (CallFunction|ConstructLogs 2.8e+03)))
    (Variables|Default|SetCurrent%20Create%20Log%20Time 0.0)
    (switch int (Variables|/Game/Blueprints/Log_BP.Log_BP_C|GetLength (Variables|Default|GetCurrent%20Log%20Created))
      (:1
        (Variables|Default|SetMax%20Create%20Log%20Time (- (Math|Random|RandomFloatinRange 1.25 1.5) _returnvalue)))
      (:2
        (Variables|Default|SetMax%20Create%20Log%20Time (- (Math|Random|RandomFloatinRange 1.5 1.75) _returnvalue)))
      (:3
        (Variables|Default|SetMax%20Create%20Log%20Time (- (Math|Random|RandomFloatinRange 2.0 2.25) _returnvalue))))))