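; Lily pad actor that bobs when jumped on and spins while the chicken stands on it.
; BeginPlay picks a random spin rate and spawns a Coin_BP at the pad's location, after a random three-way switch whose listed cases are empty.
; Tick plays a 2D sound as a jump-on begins, runs BouncingAnimation, and applies the delta-scaled local rotation while HasChickenOnTop is set.
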(event EventBeginPlay
  (|CallParentFunction)
  (Variables|Default|SetRotation (Math|Rotator|MakeRotator 0.0 0.0 (Math|Random|RandomFloatinRange -2e+01 2e+01)))
  (switch int (Math|Random|RandomInteger 3)
    (:0
      _)
    (:1
      _))
  (Game|SpawnActorfromClass "/Game/Blueprints/Coin_BP.Coin_BP_C" (Math|Transform|MakeTransform (Transformation|GetActorLocation)) "Undefined" 0 0))

(event Collision|EventActorBeginOverlap
  (params (OtherActor :type Actor%20Object%20Reference)))

(event EventTick
  (params (DeltaSeconds :type Float%20%28single-precision%29))
  (Variables|Default|SetMain%20Delta%20Seconds DeltaSeconds)
  (CallFunction|AttemptPlayJumpedonSound)
  (CallFunction|BouncingAnimation (Variables|Default|GetMain%20Delta%20Seconds))
  (if (Variables|Default|GetHas%20Chicken%20On%20Top)
    (Transformation|AddActorLocalRotation (* (Variables|Default|GetRotation) (Variables|Default|GetMain%20Delta%20Seconds)) false false)))

(fn ConstructionScript
  (|CallParentFunction))

(fn AttemptPlayJumpedonSound
  (if (and (== (Variables|Default|GetCurrent%20Jumped%20On%20Time) 0.0) (Variables|Default|GetIs%20Being%20Jumped%20On))
    (Audio|PlaySound2D "/Game/media/sounds/lily_pad.lily_pad" 1.0 1.0 0.0 0 0)))