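; Vehicle actor that drives along the X axis in either direction, set by FacingLeft, in a game with a chicken.
; BeginPlay turns it to face its direction and randomly picks a car or truck mesh, widening and shifting the collision box for trucks.
; Tick moves it by Speed, plays one random car sound the first time the chicken is near, and destroys it past the X bounds.
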(event EventBeginPlay
  (bind _staticmesh (Variables|Default|GetStaticMesh))
  (bind _box (Variables|Default|GetBox))
  (bind _box_2 (Variables|Default|GetBox))
  (bind _returnvalue (Transformation|GetWorldScale _box))
  (bind _returnvalue_2 (Transformation|GetWorldLocation _box_2))
  (if (Variables|Default|GetFacing%20Left)
    (Class|Actor|AddActorWorldRotation "0,180.000000, 0"))
  (bind _output_get (Variables|Default|SetVehicle%20Type (Math|Random|RandomInteger 8)))
  (switch int _output_get
    (:0
      (Components|StaticMesh|SetStaticMesh _staticmesh "/Game/media/meshes/car2.car2"))
    (:1
      (Components|StaticMesh|SetStaticMesh _staticmesh "/Game/media/meshes/car3.car3"))
    (:2
      (Components|StaticMesh|SetStaticMesh _staticmesh "/Game/media/meshes/car4.car4"))
    (:3
      (Components|StaticMesh|SetStaticMesh _staticmesh "/Game/media/meshes/truck.truck")
      (Transformation|SetWorldScale3D _box (Math|Vector|MakeVector (+ (.x _returnvalue) 3.0) (.y _returnvalue) (.z _returnvalue)) :!label _label)
      (if (Variables|Default|GetFacing%20Left)
        (Transformation|SetWorldLocation _box_2 (Math|Vector|MakeVector (+ (.x _returnvalue_2) 1e+02) (.y _returnvalue_2) (.z _returnvalue_2)) false false)
        (else
          (Transformation|SetWorldLocation _box_2 (Math|Vector|MakeVector (- (.x _returnvalue_2) 1e+02) (.y _returnvalue_2) (.z _returnvalue_2)) false false))))
    (:4
      (Components|StaticMesh|SetStaticMesh _staticmesh "/Game/media/meshes/truck2.truck2")
      (goto _label))
    (:5
      (Components|StaticMesh|SetStaticMesh _staticmesh "/Game/media/meshes/truck3.truck3")
      (goto _label))
    (:6
      (Components|StaticMesh|SetStaticMesh _staticmesh "/Game/media/meshes/truck4.truck4")
      (goto _label))))

(event EventTick
  (params (DeltaSeconds :type Float%20%28single-precision%29))
  (CallFunction|MoveVehicle DeltaSeconds)
  (if (Variables|Default|GetMade%20Sound)
    _
    (else
      (CallFunction|AttemptPlaySoundEffect)))
  (CallFunction|CheckifOutOfBounds))

(fn ConstructionScript)

(fn MoveVehicle
  (params (Delta%20Time :type Float%20%28single-precision%29))
  (bind _speed (Variables|Default|GetSpeed))
  (bind _returnvalue (* _speed Delta%20Time))
  (if (Variables|Default|GetFacing%20Left)
    (Transformation|AddActorWorldOffset (Math|Vector|MakeVector (* _returnvalue -1.0) 0.0 0.0))
    (else
      (Transformation|AddActorWorldOffset (Math|Vector|MakeVector _returnvalue 0.0 0.0)))))

(fn AttemptPlaySoundEffect
  (bind _chicken_ref (Variables|Default|GetChicken%20REF))
  (Utilities|IsValid _chicken_ref
    (:Is%20Valid
      (if (<= (Math|Vector|VectorLength (- (Transformation|GetActorLocation _chicken_ref) (Transformation|GetActorLocation))) 5e+02)
        (Variables|Default|SetMade%20Sound true)
        (switch int (Math|Random|RandomInteger 4)
          (:0
            (Audio|PlaySound2D "/Game/media/sounds/car_beep.car_beep" 1.0 1.0 0.0 0 0))
          (:1
            (Audio|PlaySound2D "/Game/media/sounds/car_beep2.car_beep2" 1.0 1.0 0.0 0 0))
          (:2
            (Audio|PlaySound2D "/Game/media/sounds/car_move1.car_move1" 1.0 1.0 0.0 0 0))
          (:3
            (Audio|PlaySound2D "/Game/media/sounds/car_move2.car_move2" 1.0 1.0 0.0 0 0)))))))

(fn CheckifOutOfBounds
  (if (> (Math|Float|Absolute(Float) (.x (Transformation|GetActorLocation))) 2.8e+03)
    (Actor|DestroyActor)))