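; Main camera actor that follows the player's chicken along the Y axis in Chicken Saga.
; BeginPlay caches the player pawn as a Chicken_BP and passes that reference to the GameMod_ChickenSaga_BP game mode.
; Each Tick it moves to the chicken's Y plus an offset, keeping X and height fixed, with no interpolation or sweep.
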(event EventBeginPlay
  (bind _aschicken_bp (Utilities|Casting|CastToChicken_BP (Game|Player|GetPlayerPawn 0)))
  (Variables|Default|SetChicken%20REF _aschicken_bp)
  (bind _asgame_mod_chicken_saga_bp (Utilities|Casting|CastToGameMod_ChickenSaga_BP (Game|GetGameMode)))
  (Variables|/Game/Blueprints/GameMod_ChickenSaga_BP.GameMod_ChickenSaga_BP_C|SetChicken%20REF _asgame_mod_chicken_saga_bp (Variables|Default|GetChicken%20REF)))

(event EventTick
  (params (DeltaSeconds :type Float%20%28single-precision%29))
  (Transformation|SetActorLocation (Math|Vector|MakeVector 0.0 (+ (.Y (Math|Vector|BreakVector (Transformation|GetActorLocation (Variables|Default|GetChicken%20REF)))) (Variables|Default|GetOffset%20Y)) 1.3e+03) false false))

(fn ConstructionScript)