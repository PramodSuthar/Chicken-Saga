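; Road floor chunk for a chicken road-crossing game, building one lane of road with traffic when play begins.
; It spawns left, center and right floor pieces, with only the center marked traversable, plus optional road-line props.
; A vehicle spawner is placed on a random side with matching facing and a chicken reference, and is destroyed with the chunk.
; A loop builds the row's landing nodes, attempting a coin spawn before each.
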(event EventBeginPlay
  (bind _self self)
  (bind _props (Variables|Default|GetProps))
  (bind (_transform_left _transform_mid _transform_right _y_position) (CallFunction|CalculateFloorTransform))
  (bind _returnvalue (Game|SpawnActorfromClass "/Game/Blueprints/Floor_BP.Floor_BP_C" _transform_left "Undefined" 0 1 false _self 0))
  (Variables|Default|SetLeft%20Floor _returnvalue)
  (bind _returnvalue_2 (Game|SpawnActorfromClass "/Game/Blueprints/Floor_BP.Floor_BP_C" _transform_mid "Undefined" 0 1 true _self 0))
  (Variables|Default|SetCenter%20Floor _returnvalue_2)
  (bind _returnvalue_3 (Game|SpawnActorfromClass "/Game/Blueprints/Floor_BP.Floor_BP_C" _transform_right "Undefined" 0 1 false _self 0))
  (Variables|Default|SetRight%20Floor _returnvalue_3)
  (if (Variables|Default|GetHas%20Lines)
    (bind _returnvalue_4 (Game|SpawnActorfromClass "/Game/Blueprints/RoadLines_BP.RoadLines_BP_C" (Math|Transform|MakeTransform (Math|Vector|MakeVector -2e+03 (- _y_position -1e+02) 0.0)) "Undefined" 0 true 0))
    (Utilities|Array|Add _props _returnvalue_4)
    (bind _returnvalue_5 (Game|SpawnActorfromClass "/Game/Blueprints/RoadLines_BP.RoadLines_BP_C" (Math|Transform|MakeTransform (Math|Vector|MakeVector 0.0 (- _y_position -1e+02) 0.0)) "Undefined" 0 false 0))
    (Utilities|Array|Add _props _returnvalue_5)
    (bind _returnvalue_6 (Game|SpawnActorfromClass "/Game/Blueprints/RoadLines_BP.RoadLines_BP_C" (Math|Transform|MakeTransform (Math|Vector|MakeVector 2e+03 (- _y_position -1e+02) 0.0)) "Undefined" 0 true 0))
    (Utilities|Array|Add _props _returnvalue_6))
  (CallFunction|ConstructVehicleSpawner _y_position)
  (CallFunction|ConstructLandingNodes))

(event EventTick
  (params (DeltaSeconds :type Float%20%28single-precision%29)))

(event EventDestroyed
  (for _array_element (Variables|Default|GetVehicle%20Spawners)
    (Actor|DestroyActor _array_element)))

(fn ConstructionScript
  (|CallParentFunction))

(fn ConstructVehicleSpawner
  (params (Position%20Y :type Float%20%28single-precision%29))
  (bind _output_get (LocalVariables|SetFacing%20Left (Math|Random|RandomBool)))
  (if _output_get
    (LocalVariables|SetPosition%20X 2.8e+03)
    (else
      (bind _output_get_2 (LocalVariables|SetPosition%20X -2.8e+03))))
  (bind _returnvalue (Game|SpawnActorfromClass "/Game/Blueprints/Spawn_Vehicle_BP.Spawn_Vehicle_BP_C" (Math|Transform|MakeTransform (Math|Vector|MakeVector _output_get_2 Position%20Y -1e+01)) "Undefined" 0 _output_get (Variables|Default|GetChicken_REF) 0))
  (Utilities|Array|Add (Variables|Default|GetVehicle%20Spawners) _returnvalue))

(fn ConstructLandingNodes
  (Variables|Default|SetCurrent%20Z%20Position%20for%20Landing%20Node -3e+01)
  (for _index (range 0 8)
    (CallFunction|CreateCoinAttempt)
    (CallFunction|ConstructLandingNode(FloorChunk) false)))