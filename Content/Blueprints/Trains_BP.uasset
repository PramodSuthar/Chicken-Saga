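; Train actor that travels in a straight line along the world X axis and removes itself after a set lifetime.
; The MoveLeft flag selects negative or positive X travel and, when set, rotates the actor 180 degrees at BeginPlay.
; Tick offsets the position by MoveSpeed scaled by delta time, counts LifeTime down and destroys the actor when it runs out.
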(event EventBeginPlay
  (if (Variables|Default|GetMove%20Left)
    (Transformation|SetActorRotation "0,180.000000, 0")))

(event Collision|EventActorBeginOverlap
  (params (OtherActor :type Actor%20Object%20Reference)))

(event EventTick
  (params (DeltaSeconds :type Float%20%28single-precision%29))
  (bind _move_speed (Variables|Default|GetMove%20Speed))
  (bind _returnvalue (* _move_speed DeltaSeconds))
  (if (Variables|Default|GetMove%20Left)
    (Transformation|AddActorWorldOffset (Math|Vector|MakeVector (* _returnvalue -1.0) 0.0 0.0))
    (else
      (Transformation|AddActorWorldOffset (Math|Vector|MakeVector _returnvalue 0.0 0.0))))
  (bind _output_get (Variables|Default|SetLife%20Time (- (Variables|Default|GetLife%20Time) DeltaSeconds)))
  (if (<= _output_get 0.0)
    (Actor|DestroyActor)))

(fn ConstructionScript)